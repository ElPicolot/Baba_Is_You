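; Chessboard actor that builds an 8x8 checkered board procedurally in its Construction Script.
; A single loop over 64 indices adds a static mesh component per square, deriving its grid position at 400-unit spacing from integer division and modulo.
; An XOR of row and column parity picks the black or default basic wall material for each square.
; The event graph has no active logic.
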(fn `UserConstructionScript`
  (for _index (range 64)
    (`|ExecutionSequence`
      (:`then_0`
        (bind _returnvalue (`AddComponent|NODE_AddStaticMeshComponent-0` :`RelativeTransform` (`KismetMathLibrary.Conv_VectorToTransform` (`KismetMathLibrary.MakeVector` (`KismetMathLibrary.Conv_IntToDouble` (* (/ _index 8) 400)) (`KismetMathLibrary.Conv_IntToDouble` (* (mod _index 8) 400))))))
        (`PrimitiveComponent.SetMaterial` _returnvalue 0 (select `bool` (xor (`KismetMathLibrary.Conv_IntToBool` (mod _index 2)) (`KismetMathLibrary.Conv_IntToBool` (mod (/ _index 8) 2))) :`false` "/Game/VRAC/StarterContent/Materials/M_Basic_Wall.M_Basic_Wall" :`true` "/Game/VRAC/StarterContent/Materials/M_Basic_Wall_Black.M_Basic_Wall_Black" :!type "Material Object Reference"))))))