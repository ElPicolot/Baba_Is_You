(event `self.ReceiveActorBeginOverlap`
  (params (OtherActor :type "Actor Object Reference"))
  (`|ExecutionSequence`
    (:`then_0`
      (cast `/Game/PROPRE/BABA_BP` OtherActor)
      (set `self.BABA` true))
    (:`then_1`
      (cast `/Game/PROPRE/WALL_BP` OtherActor)
      (set `self.WALL` true))
    (:`then_2`
      (cast `/Game/PROPRE/OPEN_BP` OtherActor)
      (set `self.OPEN` true))
    (:`then_3`
      (cast `/Game/PROPRE/PUSH_BP` OtherActor)
      (set `self.PUSH` true))
    (:`then_4`
      (cast `/Game/PROPRE/STOP_BP` OtherActor)
      (set `self.STOP` true))
    (:`then_5`
      (cast `/Game/PROPRE/FLAG_BP` OtherActor)
      (set `self.FLAG` true))
    (:`then_6`
      (cast `/Game/PROPRE/YOU_BP` OtherActor)
      (set `self.YOU` true))))

(event `self.ReceiveActorEndOverlap`
  (params (OtherActor :type "Actor Object Reference"))
  (`|ExecutionSequence`
    (:`then_0`
      (cast `/Game/PROPRE/BABA_BP` OtherActor)
      (set `self.BABA` false))
    (:`then_1`
      (cast `/Game/PROPRE/WALL_BP` OtherActor)
      (set `self.WALL` false))
    (:`then_2`
      (cast `/Game/PROPRE/OPEN_BP` OtherActor)
      (set `self.OPEN` false))
    (:`then_3`
      (cast `/Game/PROPRE/PUSH_BP` OtherActor)
      (set `self.PUSH` false))
    (:`then_4`
      (cast `/Game/PROPRE/STOP_BP` OtherActor)
      (set `self.STOP` false))
    (:`then_5`
      (cast `/Game/PROPRE/FLAG_BP` OtherActor)
      (set `self.FLAG` false))
    (:`then_6`
      (cast `/Game/PROPRE/YOU_BP` OtherActor)
      (set `self.YOU` false))))

(event `self.ReceiveTick`
  (params (DeltaSeconds :type "Float (single-precision)"))
  (`|ExecutionSequence`
    (:`then_0`
      (`|ExecutionSequence`
        (:`then_0`
          (if (`self.BABA`)
            (`KismetSystemLibrary.PrintString` "IS:             BABA" true true (struct :`R` 0.532916 :`B` 1.0 :`A` 1.0))))
        (:`then_1`
          (if (`self.WALL`)
            (`KismetSystemLibrary.PrintString` "IS:           WALL" true true (struct :`R` 0.532916 :`B` 1.0 :`A` 1.0))))
        (:`then_2`
          (if (`self.OPEN`)
            (`KismetSystemLibrary.PrintString` "IS:          OPEN" true true (struct :`R` 0.532916 :`B` 1.0 :`A` 1.0))))
        (:`then_3`
          (if (`self.PUSH`)
            (`KismetSystemLibrary.PrintString` "IS:          PUSH" true true (struct :`R` 0.532916 :`B` 1.0 :`A` 1.0))))
        (:`then_4`
          (if (`self.STOP`)
            (`KismetSystemLibrary.PrintString` "IS:          STOP" true true (struct :`R` 0.532916 :`B` 1.0 :`A` 1.0))))
        (:`then_5`
          (if (`self.FLAG`)
            (`KismetSystemLibrary.PrintString` "IS:          FLAG" true true (struct :`R` 0.532916 :`B` 1.0 :`A` 1.0))))
        (:`then_6`
          (if (`self.YOU`)
            (`KismetSystemLibrary.PrintString` "IS:         YOU" true true (struct :`R` 0.532916 :`B` 1.0 :`A` 1.0))))))
    (:`then_1`
      (if (and (`self.STOP`) (`self.BABA`))
        (`KismetSystemLibrary.PrintString` "BABA STOP MOVING")))
    (:`then_2`
      (if true
        _))))

(event `self.Box.OnComponentBeginOverlap`
  (params (OverlappedComponent :type "PrimitiveComponent Object Reference") (OtherActor :type "Actor Object Reference") (OtherComp :type "PrimitiveComponent Object Reference") (OtherBodyIndex :type Integer) (bFromSweep :type Boolean) (SweepResult :type "HitResult Structure (by ref)"))
  (cast `/Game/ThirdPerson/Blueprints/BP_ThirdPersonCharacter` OtherActor)
  (`KismetSystemLibrary.PrintString` "toucher perso"))

(event `self.NewFunction`)

(fn `UserConstructionScript`)