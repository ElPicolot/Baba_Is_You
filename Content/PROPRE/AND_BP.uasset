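; AND_BP is an actor that detects overlaps with the player and with flag and push cubes, apparently as an AND piece in a cube puzzle.
; On actor overlap, a Sequence casts the other actor to BP_ThirdPersonCharacter, Cubesimple_flag and Cubesimple_push, printing a debug string for each match.
; A Box component separately reports character contact.
; It only prints messages so far, with an empty NewFunction event and leftover unconnected nodes.
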(event `self.ReceiveActorBeginOverlap`
  (params (OtherActor :type "Actor Object Reference"))
  (`|ExecutionSequence`
    (:`then_0`
      (cast `/Game/ThirdPerson/Blueprints/BP_ThirdPersonCharacter` OtherActor)
      (`KismetSystemLibrary.PrintString` "toucher_Cube_Push" true true (struct :`R` 0.97139 :`G` 1.0 :`A` 1.0)))
    (:`then_1`
      (cast `/Game/VRAC/Object/Cubesimple_flag` OtherActor)
      (`KismetSystemLibrary.PrintString` "IS_FLAG" true true (struct :`R` 0.87549 :`G` 1.0 :`A` 1.0)))
    (:`then_2`
      (cast `/Game/VRAC/Object/Cubesimple_push` OtherActor)
      (`KismetSystemLibrary.PrintString` "IS_PUSH" true true (struct :`R` 0.958818 :`G` 1.0 :`A` 1.0)))
    (:`then_3`
      (cast `/Game/ThirdPerson/Blueprints/BP_ThirdPersonCharacter` OtherActor)
      (`KismetSystemLibrary.PrintString` "lalalal" true true (struct :`R` 0.959213 :`G` 1.0 :`A` 1.0)))))

(event `self.Box.OnComponentBeginOverlap`
  (params (OverlappedComponent :type "PrimitiveComponent Object Reference") (OtherActor :type "Actor Object Reference") (OtherComp :type "PrimitiveComponent Object Reference") (OtherBodyIndex :type Integer) (bFromSweep :type Boolean) (SweepResult :type "HitResult Structure (by ref)"))
  (cast `/Game/ThirdPerson/Blueprints/BP_ThirdPersonCharacter` OtherActor)
  (`KismetSystemLibrary.PrintString` "toucher perso"))

(event `self.NewFunction`)

(fn `UserConstructionScript`)