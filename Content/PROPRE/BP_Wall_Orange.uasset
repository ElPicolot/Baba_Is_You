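; BP_Wall_Orange is an orange wall actor, apparently a word-block puzzle prototype, that only reports what touches it through debug messages.
; Actor overlap runs a Sequence of casts to the third-person character, AND_BP and IS_BP, printing a colored message for each match.
; A separate Box component overlap also prints when the character enters.
; Construction script and NewFunction are empty, and several cast-and-print chains, including flag and push cube checks, are disconnected.
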(event `self.ReceiveActorBeginOverlap`
  (params (OtherActor :type "Actor Object Reference"))
  (`|ExecutionSequence`
    (:`then_0`
      (cast `/Game/ThirdPerson/Blueprints/BP_ThirdPersonCharacter` OtherActor)
      (`KismetSystemLibrary.PrintString` "toucher_Cube_Push" true true (struct :`R` 0.97139 :`G` 1.0 :`A` 1.0)))
    (:`then_1`
      (cast `/Game/PROPRE/AND_BP` OtherActor)
      (`KismetSystemLibrary.PrintString` "ANDBABA" true true (struct :`R` 1.0 :`B` 0.305423 :`A` 1.0)))
    (:`then_3`
      (cast `/Game/PROPRE/IS_BP` OtherActor)
      (`KismetSystemLibrary.PrintString` "WALL IS" true true (struct :`R` 0.575896 :`G` 1.0 :`A` 1.0)))))

(event `self.Box.OnComponentBeginOverlap`
  (params (OverlappedComponent :type "PrimitiveComponent Object Reference") (OtherActor :type "Actor Object Reference") (OtherComp :type "PrimitiveComponent Object Reference") (OtherBodyIndex :type Integer) (bFromSweep :type Boolean) (SweepResult :type "HitResult Structure (by ref)"))
  (cast `/Game/ThirdPerson/Blueprints/BP_ThirdPersonCharacter` OtherActor)
  (`KismetSystemLibrary.PrintString` "toucher perso"))

(event `self.NewFunction`)

(fn `UserConstructionScript`)