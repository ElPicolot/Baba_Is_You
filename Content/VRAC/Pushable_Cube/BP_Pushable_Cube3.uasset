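; BP_Pushable_Cube3 is a prototype pushable cube that detects interaction with the third-person character but only prints debug messages and does not yet move.
; It caches the character on BeginPlay, and overlaps on its Fwd component set or clear the character's CanInteractBox flag without filtering the overlapping actor.
; While both interaction flags are true, Tick reads ForwardBackwardAxis and prints whether input is idle, forward or backward.
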(event `self.ReceiveBeginPlay`
  (bind _returnvalue (`GameplayStatics.GetActorOfClass` "/Game/ThirdPerson/Blueprints/BP_ThirdPersonCharacter.BP_ThirdPersonCharacter_C"))
  (set `self.CharacterREF` _returnvalue))

(event `self.ReceiveTick`
  (params (DeltaSeconds :type "Float (single-precision)"))
  (bind _forward_backward_axis (`/Game/ThirdPerson/Blueprints/BP_ThirdPersonCharacter.Forward Backward Axis` (`self.CharacterREF`)))
  (if (`/Game/ThirdPerson/Blueprints/BP_ThirdPersonCharacter.IsInteractibleBox?` (`self.CharacterREF`))
    (if (`/Game/ThirdPerson/Blueprints/BP_ThirdPersonCharacter.CanInteractBox?` (`self.CharacterREF`))
      (`|ExecutionSequence`
        (:`then_0`
          (if (== _forward_backward_axis 0.0)
            (`KismetSystemLibrary.PrintString` "is not moving forward or backwards" true true (struct :`R` 0.066037 :`B` 1.0 :`A` 1.0))
            (elif (>= _forward_backward_axis 0.1)
              (`KismetSystemLibrary.PrintString` "Is moving forward" true true (struct :`R` 0.040547 :`G` 1.0 :`A` 1.0))
              (else
                (`KismetSystemLibrary.PrintString` "Is moving backward" true true (struct :`R` 0.040547 :`G` 1.0 :`A` 1.0))))))))))

(event `self.Fwd.OnComponentBeginOverlap`
  (params (OverlappedComponent :type "PrimitiveComponent Object Reference") (OtherActor :type "Actor Object Reference") (OtherComp :type "PrimitiveComponent Object Reference") (OtherBodyIndex :type Integer) (bFromSweep :type Boolean) (SweepResult :type "HitResult Structure (by ref)"))
  (`KismetSystemLibrary.PrintString` "Is Overlap You ?" true true (struct :`R` 0.741778 :`G` 1.0 :`A` 1.0))
  (set `/Game/ThirdPerson/Blueprints/BP_ThirdPersonCharacter.CanInteractBox?` true (`self.CharacterREF`)))

(event `self.Fwd.OnComponentEndOverlap`
  (params (OverlappedComponent :type "PrimitiveComponent Object Reference") (OtherActor :type "Actor Object Reference") (OtherComp :type "PrimitiveComponent Object Reference") (OtherBodyIndex :type Integer))
  (`KismetSystemLibrary.PrintString` "DOne " true true (struct :`G` 0.517005 :`B` 1.0 :`A` 1.0))
  (set `/Game/ThirdPerson/Blueprints/BP_ThirdPersonCharacter.CanInteractBox?` false (`self.CharacterREF`)))

(fn `UserConstructionScript`)